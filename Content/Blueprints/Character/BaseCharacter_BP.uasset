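; BaseCharacter_BP is the player character, with a held self-heal ability, animation control, death and respawn.
; Ability1 toggles heal particles, the attack animation flag and movement, while Tick repeats the AbilityManager heal on a timer as the key is held.
; Tick also drives Grunt_ABP running and triggers Death once at zero health.
; During play, death leads to a delayed respawn that spawns and possesses a fresh character at the first PlayerStart.
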(event `InputAction|Ability1`
  (params (Key :type "Key Structure"))
  (bind _characterdead (`self.CharacterDead`))
  (bind _returnvalue (`AbilityManagerComponent.GetAbility` (`self.AbilityManager`) "EHeal"))
  ;[1 1 1] Input Attack
  (:`Pressed`
    (if (not _characterdead)
      (`/Engine/EditorBlueprintResources/StandardMacros.IsValid` _returnvalue
        (:`Is Valid`
          (set `self.IsHoldingAbility1` true)
          (`self.Start SelfHealAnimation`)))))
  (:`Released`
    (if (not _characterdead)
      (`/Engine/EditorBlueprintResources/StandardMacros.IsValid` _returnvalue
        (:`Is Valid`
          (set `self.IsHoldingAbility1` false)
          (`self.Finish SelfHealAnimation`))))))

(event `self.ReceiveTick`
  (params (DeltaSeconds :type "Float (single-precision)"))
  (bind _returnvalue (`AbilityManagerComponent.GetAbility` (`self.AbilityManager`) "EHeal"))
  ;[1 1 1] Update
  (bind _asto_the_top_game_mode_base_bp (cast `/Game/Blueprints/ToTheTopGameModeBase_BP` (`GameplayStatics.GetGameMode`)))
  (if (`|EnumEquality` (`ToTheTopGameModeBase.GetGameState` _asto_the_top_game_mode_base_bp) "EPlaying")
    (bind _asbase_character_bp (cast `/Game/Blueprints/Character/BaseCharacter_BP` (`GameplayStatics.GetPlayerCharacter` 0)))
    (if (> (`BaseCharacter.health` _asbase_character_bp) 0)
      (`/Engine/EditorBlueprintResources/StandardMacros.IsValid` _returnvalue
        (:`Is Valid`
          (if (`PlayerController.IsInputKeyDown` (`GameplayStatics.GetPlayerController` 0) (stale `InputAction|Ability1` Key))
            (bind _output_get (set `self.timeBetweenAttacks` (- (`self.timeBetweenAttacks`) DeltaSeconds)))
            (if (<= _output_get 0.0)
              (`Ability.Execute` _returnvalue)
              (set `self.timeBetweenAttacks` 1.0))
            (else
              (`self.Movement Animation` :!label _label))))
        (:`Is Not Valid`
          (goto _label)))
      (else
        (`/Engine/EditorBlueprintResources/StandardMacros.DoOnce` false
          (:`Completed`
            (`self.Death` _asbase_character_bp)))))
    (else
      (bind _asgrunt_abp (cast `/Game/Blueprints/Character/Grunt_ABP` (`SkeletalMeshComponent.GetAnimInstance` (`self.Mesh`))))
      (set `/Game/Blueprints/Character/Grunt_ABP.CanRun` false _asgrunt_abp))))

(event `self.InjuredAnimation`
  ;[1 1 1] Injured Animation
  (bind _asgrunt_abp (cast `/Game/Blueprints/Character/Grunt_ABP` (`SkeletalMeshComponent.GetAnimInstance` (`self.Mesh`))))
  (set `/Game/Blueprints/Character/Grunt_ABP.hasBeenInjured` true _asgrunt_abp)
  (`KismetSystemLibrary.Delay` 1.0)
  (set `/Game/Blueprints/Character/Grunt_ABP.hasBeenInjured` false _asgrunt_abp))

(event `self.DeathAnimation`
  ;[1 1 1] Death Animation
  (bind _asgrunt_abp (cast `/Game/Blueprints/Character/Grunt_ABP` (`SkeletalMeshComponent.GetAnimInstance` (`self.Mesh`))))
  (set `/Game/Blueprints/Character/Grunt_ABP.isDead` true _asgrunt_abp)
  (`CharacterMovementComponent.DisableMovement` (`self.CharacterMovement`)))

(event `self.Death`
  ;[1 1 1] Death
  (set `self.CharacterDead` true)
  (bind _asbase_character_bp (cast `/Game/Blueprints/Character/BaseCharacter_BP` (`GameplayStatics.GetPlayerCharacter` 0)))
  (`self.DeathAnimation` _asbase_character_bp)
  (`KismetSystemLibrary.Delay` (`self.DeathAnimationLength`))
  (bind _asto_the_top_game_mode_base_bp (cast `/Game/Blueprints/ToTheTopGameModeBase_BP` (`GameplayStatics.GetGameMode`)))
  (if (`|EnumEquality` (`ToTheTopGameModeBase.GetGameState` _asto_the_top_game_mode_base_bp) "EPlaying")
    (`KismetSystemLibrary.Delay` (`self.RepawnDelay`))
    (`self.Respawn Character`)))

(fn `Finish SelfHealAnimation`
  (bind _returnvalue (`AbilityManagerComponent.GetAbility` (`self.AbilityManager`) "EHeal"))
  (`/Engine/EditorBlueprintResources/StandardMacros.IsValid` _returnvalue
    (:`Is Valid`
      (bind _asheal_self (cast `HealSelf` _returnvalue))
      (bind _asgrunt_abp (cast `/Game/Blueprints/Character/Grunt_ABP` (`SkeletalMeshComponent.GetAnimInstance` (`self.Mesh`))))
      (set `/Game/Blueprints/Character/Grunt_ABP.IsAttacking` false _asgrunt_abp)
      (`SceneComponent.SetVisibility` (`HealSelf.HealParticleSystem` _asheal_self) false false)
      (`CharacterMovementComponent.SetMovementMode` (`self.CharacterMovement`) "MOVE_Walking" 0))))

(fn `Movement Animation`
  (bind _returnvalue (`SkeletalMeshComponent.GetAnimInstance` (`self.Mesh`)))
  (if (or (!= (`self.GetInputAxisValue`) 0.0) (!= (`self.GetInputAxisValue`) 0.0))
    (bind _asgrunt_abp (cast `/Game/Blueprints/Character/Grunt_ABP` _returnvalue))
    (set `/Game/Blueprints/Character/Grunt_ABP.CanRun` true _asgrunt_abp)
    (else
      (bind _asgrunt_abp_2 (cast `/Game/Blueprints/Character/Grunt_ABP` _returnvalue))
      (set `/Game/Blueprints/Character/Grunt_ABP.CanRun` false _asgrunt_abp_2))))

(fn `Respawn Character`
  (`self.K2_DestroyActor`)
  (set `self.CharacterDead` false)
  (bind _outactors (`GameplayStatics.GetAllActorsOfClass` "/Script/Engine.PlayerStart"))
  (if (`KismetArrayLibrary.Array_IsValidIndex` _outactors)
    (bind _returnvalue (`|SpawnActorFromClass` "BaseCharacter_BP_C" (`KismetMathLibrary.Conv_VectorToTransform` (`self.K2_GetActorLocation` (`|GetArrayItem` _outactors))) "Undefined" "OverrideRootScale" null null))
    (`Controller.Possess` (`GameplayStatics.GetPlayerController` 0) _returnvalue)))

(fn `Start SelfHealAnimation`
  (bind _charactermovement (`self.CharacterMovement`))
  (bind _returnvalue (`AbilityManagerComponent.GetAbility` (`self.AbilityManager`) "EHeal"))
  (`/Engine/EditorBlueprintResources/StandardMacros.IsValid` _returnvalue
    (:`Is Valid`
      (bind _asheal_self (cast `HealSelf` _returnvalue))
      (bind _asgrunt_abp (cast `/Game/Blueprints/Character/Grunt_ABP` (`SkeletalMeshComponent.GetAnimInstance` (`self.Mesh`))))
      (`SceneComponent.SetVisibility` (`HealSelf.HealParticleSystem` _asheal_self) true false)
      (set `/Game/Blueprints/Character/Grunt_ABP.IsAttacking` true _asgrunt_abp)
      (`MovementComponent.StopMovementImmediately` _charactermovement)
      (`CharacterMovementComponent.DisableMovement` _charactermovement))))

(fn `UserConstructionScript`)