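; Spike trap actor that repeatedly drains health from the player while its damage box is occupied.
; A BaseCharacter_BP entering DamageBox sets IsDamaging, and any end overlap clears it.
; Tick counts down an interval timer, then damages player character 0, rather than the stored overlapping actor, and resets the timer.
; The countdown runs even when idle, so damage can land immediately on entry.
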(event `self.ReceiveTick`
  (params (DeltaSeconds :type "Float (single-precision)"))
  (bind _returnvalue (- (`self.DamageIntervalTimer`) DeltaSeconds))
  ;[1 1 1] Damage Player
  (set `self.DamageIntervalTimer` _returnvalue)
  (if (<= _returnvalue 0.0)
    (if (`self.isDamaging`)
      (bind _asbase_character_bp (cast `/Game/Blueprints/Character/BaseCharacter_BP` (`GameplayStatics.GetPlayerCharacter` 0)))
      (`BaseCharacter.AddHealth` _asbase_character_bp -10)
      (set `self.DamageIntervalTimer` 1.0))))

(event `self.Damage Box.OnComponentBeginOverlap`
  (params (OverlappedComponent :type "PrimitiveComponent Object Reference") (OtherActor :type "Actor Object Reference") (OtherComp :type "PrimitiveComponent Object Reference") (OtherBodyIndex :type Integer) (bFromSweep :type Boolean) (SweepResult :type "HitResult Structure (by ref)"))
  (cast `/Game/Blueprints/Character/BaseCharacter_BP` OtherActor)
  (set `self.isDamaging` true))

(event `self.Damage Box.OnComponentEndOverlap`
  (params (OverlappedComponent :type "PrimitiveComponent Object Reference") (OtherActor :type "Actor Object Reference") (OtherComp :type "PrimitiveComponent Object Reference") (OtherBodyIndex :type Integer))
  (set `self.isDamaging` false))

(fn `UserConstructionScript`)