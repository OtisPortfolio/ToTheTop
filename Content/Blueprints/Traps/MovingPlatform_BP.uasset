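; Moving platform Blueprint that shuttles its static mesh back and forth between its starting point and an EndLocation marker.
; BeginPlay caches both world positions, then Tick accumulates time and lerps the mesh over Interval seconds, flipping IsForward at each end.
; The cached world positions are applied through SetRelativeLocation, without sweep, so they only line up when relative and world space coincide.
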(event `self.ReceiveBeginPlay`
  ;[1 1 1] Set Start and End locations
  (set `self.StartLoc` (`SceneComponent.K2_GetComponentLocation` (`self.StaticMeshComponent`)))
  (set `self.EndLoc` (`SceneComponent.K2_GetComponentLocation` (`self.End Location`))))

(event `self.ReceiveTick`
  (params (DeltaSeconds :type "Float (single-precision)"))
  ;[1 1 1] Move Platform
  (set `self.Alpha` (+ DeltaSeconds (`self.Alpha`)))
  (if (`self.IsForward`)
    (`SceneComponent.K2_SetRelativeLocation` (`self.StaticMeshComponent`) (`KismetMathLibrary.VLerp` (`self.StartLoc`) (`self.EndLoc`) (/ (`self.Alpha`) (`self.Interval`))) false false)
    (if (> (`self.Alpha`) (`self.Interval`))
      (set `self.Alpha` 0.0)
      (set `self.IsForward` false))
    (else
      (`SceneComponent.K2_SetRelativeLocation` (`self.StaticMeshComponent`) (`KismetMathLibrary.VLerp` (`self.EndLoc`) (`self.StartLoc`) (/ (`self.Alpha`) (`self.Interval`))) false false)
      (if (> (`self.Alpha`) (`self.Interval`))
        (set `self.Alpha` 0.0)
        (set `self.IsForward` true)))))

(fn `UserConstructionScript`)