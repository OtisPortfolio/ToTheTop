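; Blade trap actor that moves its Cone component back and forth between its root position and an EndLocation component.
; BeginPlay caches both world locations, and Tick accumulates delta time to lerp between them, with separate intervals for the forward and return strokes.
; A one-second Delay inside Tick pauses the blade at each end before flipping direction.
; The cached world positions are applied as the Cone's relative location.
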(event `self.ReceiveBeginPlay`
  ;[1 1 1] Set Start and End locations
  (set `self.StartLoc` (`SceneComponent.K2_GetComponentLocation` (`self.DefaultSceneRoot`)))
  (set `self.EndLoc` (`SceneComponent.K2_GetComponentLocation` (`self.End Location`))))

(event `self.ReceiveTick`
  (params (DeltaSeconds :type "Float (single-precision)"))
  ;[1 1 1] Move Blade
  (set `self.Alpha` (+ DeltaSeconds (`self.Alpha`)))
  (if (`self.IsForward`)
    (if (> (`self.Alpha`) (`self.UpInterval`))
      (`KismetSystemLibrary.Delay` 1.0 :!label _label)
      (set `self.Alpha` 0.0)
      (set `self.IsForward` (not (`self.isForward`)))
      (else
        (if (`self.IsForward`) :!label _label_2
          (`SceneComponent.K2_SetRelativeLocation` (`self.Cone`) (`KismetMathLibrary.VLerp` (`self.StartLoc`) (`self.EndLoc`) (/ (`self.Alpha`) (`self.UpInterval`))) false false)
          (else
            (`SceneComponent.K2_SetRelativeLocation` (`self.Cone`) (`KismetMathLibrary.VLerp` (`self.EndLoc`) (`self.StartLoc`) (/ (`self.Alpha`) (`self.DownInterval`))) false false)))))
    (elif (> (`self.Alpha`) (`self.DownInterval`))
      (goto _label)
      (else
        (goto _label_2)))))

(fn `UserConstructionScript`)